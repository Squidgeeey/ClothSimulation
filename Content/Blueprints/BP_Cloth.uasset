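; BP_Cloth is an interactive cloth actor with keyboard controls and a wind indicator.
; Each Tick points an arrow along WindVector, stretching it by wind strength, and feeds a clamped constriction amount to ConstrictCloth.
; Held Left and Right keys set the rate that changes that amount.
; L calls ReleaseCloth, while R calls ResetCloth and resets the amount, which the next Tick clamps.
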(event EventBeginPlay)

(event Collision|EventActorBeginOverlap
  (params (OtherActor :type Actor%20Object%20Reference)))

(event EventTick
  (params (DeltaSeconds :type Float%20%28single-precision%29))
  (bind _windvector (Variables|Default|GetWindVector))
  (Utilities|FlowControl|Sequence
    (:then_0
      (Transformation|SetWorldRotation (Variables|Default|GetArrowRoot) (Math|Conversions|RotationFromXVector _windvector) false false)
      (Transformation|SetWorldScale3D (Variables|Default|GetArrow) (Math|Vector|MakeVector (/ (Math|Vector|VectorLength _windvector) 5.0) 1.5 1.5)))
    (:then_1
      (bind _output_get (Variables|Default|SetConstrictedAmount (Math|Float|Clamp(Float) (+ (Variables|Default|GetConstrictedAmount) (* (Variables|Default|GetConstrictingRate) DeltaSeconds)) 0.2 0.8)))
      (Class|Cloth|ConstrictCloth _output_get))))

(event Input|KeyboardEvents|L
  (params (Key :type Key%20Structure :default "None"))
  (:Pressed
    (Class|Cloth|ReleaseCloth)))

(event Input|KeyboardEvents|Left
  (params (Key :type Key%20Structure :default "None"))
  (:Pressed
    (Variables|Default|SetConstrictingRate -1.0))
  (:Released
    (Variables|Default|SetConstrictingRate 0.0)))

(event Input|KeyboardEvents|Right
  (params (Key :type Key%20Structure :default "None"))
  (:Pressed
    (Variables|Default|SetConstrictingRate 1.0))
  (:Released
    (Variables|Default|SetConstrictingRate 0.0)))

(event Input|KeyboardEvents|R
  (params (Key :type Key%20Structure :default "None"))
  (:Pressed
    (Class|Cloth|ResetCloth)
    (Variables|Default|SetConstrictedAmount 1.0)))

(fn ConstructionScript)